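; Blueprint interface that showcase setup assets implement to describe themselves to a showcase system.
; It exposes getters for indexed cameras and their count, a slot number and a display name.
; Further getters supply UI control definitions: general showcase controls, sliders, twin sliders, checkboxes, button lists and separators.
; The interface only declares functions; implementers provide all data and behavior.
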(fn `GetButtonListControls`
  (returns (ButtonListControls :type "Array of /Game/MyContent/VigilanteContent/Shared/Blueprints/Showcase/Component/FButtonsControls Structure"))
  (return))

(fn `GetCheckboxControls`
  (returns (CheckboxControls :type "Array of /Game/MyContent/VigilanteContent/Shared/Blueprints/Showcase/Component/FCheckboxControls Structure"))
  (return))

(fn `GetSeparators`
  (returns (Separators :type "Array of /Game/MyContent/VigilanteContent/Shared/Blueprints/Showcase/Component/FSeparator Structure"))
  (return))

(fn `GetShowcaseCamera`
  (params (Index :type Integer))
  (returns (Camera :type "CameraActor Object Reference"))
  (return null))

(fn `GetShowcaseCameraCount`
  (returns (Count :type Integer))
  (return 0))

(fn `GetShowcaseControls`
  (returns (ControlsInterface :type "/Game/MyContent/VigilanteContent/Shared/Blueprints/Showcase/Interfaces/BP_ShowcaseControlsInterface Interface"))
  (return null))

(fn `GetShowcaseName`
  (returns (Name :type String))
  (return ""))

(fn `GetShowcaseSlot`
  (returns (Slot :type Integer))
  (return 0))

(fn `GetSliderControls`
  (returns (SliderControls :type "Array of /Game/MyContent/VigilanteContent/Shared/Blueprints/Showcase/Component/FSliderControls Structure"))
  (return))

(fn `GetTwinSliderControls`
  (returns (TwinSliderControls :type "Array of /Game/MyContent/VigilanteContent/Shared/Blueprints/Showcase/Component/FTwinSliderControls Structure"))
  (return))